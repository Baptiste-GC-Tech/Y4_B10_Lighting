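; BP_Door is a Sector 1 door that opens once two linked lights are both activated.
; Each tick it polls LightActivated on Light1 and Light2 until both are true, then latches DoorOpened so the opening fires only once.
; OpenDoor plays a timeline that swings the Scene component about its roll axis to -95 degrees, with no logic to close it again.
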(event Custom|OpenDoor
  (bind _alpha (Timeline|TL_Opendoor Play)
    (:Update
      (Transformation|SetRelativeRotation (Variables|Default|GetScene) (Math|Rotator|MakeRotator (Math|Float|Lerp 0.0 -95.0 _alpha) 0.0 0.0) false false))))

(event EventTick
  (params (DeltaSeconds :type Float%20%28single-precision%29))
  (if (not (Variables|Default|GetDoorOpened))
    (if (Variables|/Game/Sector1/BP_DoorLight1.BP_DoorLight1_C|GetLightActivated (Variables|Default|GetLight1))
      (if (Variables|/Game/Sector1/BP_DoorLight2.BP_DoorLight2_C|GetLightActivated (Variables|Default|GetLight2))
        (Variables|Default|SetDoorOpened true)
        (CallFunction|OpenDoor)))))

(fn ConstructionScript)