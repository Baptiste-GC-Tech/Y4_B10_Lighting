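; BP_Generator is an interactable generator that can be repaired to activate a door light in its sector.
; Interact checks the Sector1 flag, then Sector2, to choose between DoorLight1 and DoorLight2, and does nothing if neither is set.
; Either branch first runs FixGenerator, which plays a 2D repair sound and deactivates four Niagara effects.
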(event Custom|FixGenerator
  (Audio|SpawnSound2D "/Game/Sector1/SFX/RepairSFX.RepairSFX" 1.0 1.0 0.0 0)
  (Components|Activation|SetActive (Variables|Default|GetNiagara) false false)
  (Components|Activation|SetActive (Variables|Default|GetNiagara1) false false)
  (Components|Activation|SetActive (Variables|Default|GetNiagara2) false false)
  (Components|Activation|SetActive (Variables|Default|GetNiagara3) false false))

(event Custom|ActivateLamp2
  (Default|ActivateLight (Variables|Default|GetDoorLight_2)))

(event Custom|ActivateLamp1
  (Default|ActivateLight (Variables|Default|GetDoorLight_1)))

(event EventInteract
  (if (Variables|Default|GetSector1)
    (CallFunction|FixGenerator)
    (CallFunction|ActivateLamp1)
    (elif (Variables|Default|GetSector2)
      (CallFunction|FixGenerator)
      (CallFunction|ActivateLamp2))))

(fn ConstructionScript)