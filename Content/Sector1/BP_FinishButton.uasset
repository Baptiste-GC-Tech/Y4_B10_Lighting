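; BP_FinishButton is an interactable Blueprint that ends the current run and restarts the level.
; Interact calls EndGame, which casts player 0's pawn to BP_FirstPersonCharacter, sets its EndWidget to Hidden and disables player input.
; After a short delay, it reloads the current level by name.
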(event Custom|EndGame
  (bind _returnvalue (Game|GetPlayerController 0))
  (bind _asbp_first_person_character (Utilities|Casting|CastToBP_FirstPersonCharacter (Game|GetPlayerCharacter 0)))
  (Widget|SetVisibility (Variables|/Game/FirstPerson/Blueprints/BP_FirstPersonCharacter.BP_FirstPersonCharacter_C|GetEndWidget _asbp_first_person_character) "Hidden")
  (Input|DisableInput _returnvalue _returnvalue)
  (Utilities|FlowControl|Delay 5.0)
  (bind _returnvalue_2 (Game|GetCurrentLevelName true))
  (Game|OpenLevel(byName) (Utilities|String|StringToName _returnvalue_2)))

(event EventInteract
  (CallFunction|EndGame))

(fn ConstructionScript)